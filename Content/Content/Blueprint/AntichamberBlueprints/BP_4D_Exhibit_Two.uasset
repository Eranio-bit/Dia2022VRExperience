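; BP_4D_Exhibit_Two is an Antichamber-style exhibit that links two objects' materials to the world positions of two poles.
; On BeginPlay it fills pole and object arrays, then pairs each object with two neighboring poles, wrapping around so each object receives the poles in opposite order.
; Each object gets a dynamic material instance with those locations passed once as Pole1 and Pole2 vector parameters.
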(event `self.ReceiveBeginPlay`
  (`KismetArrayLibrary.Array_Add` (`self.PoleArray`) (`self.Pole0`))
  (`KismetArrayLibrary.Array_Add` (`self.PoleArray`) (`self.Pole1`))
  (`KismetArrayLibrary.Array_Add` (`self.ObjectArray`) (`self.Object1`))
  (`KismetArrayLibrary.Array_Add` (`self.ObjectArray`) (`self.Object2`))
  (if (== (`KismetArrayLibrary.Array_Length` (`self.PoleArray`)) (`KismetArrayLibrary.Array_Length` (`self.ObjectArray`)))
    (for _index (range (+ (`KismetArrayLibrary.Array_LastIndex` (`self.PoleArray`)) 1))
      (`self.CreateAndSetMaterial` (`|GetArrayItem` (`self.PoleArray`) (mod (+ _index 1) (`KismetArrayLibrary.Array_Length` (`self.PoleArray`)))) (`|GetArrayItem` (`self.PoleArray`) _index) (`|GetArrayItem` (`self.ObjectArray`) _index)))))

(fn `CreateAndSetMaterial`
  (params (Pole0 :type "SceneComponent Object Reference") (Pole1 :type "SceneComponent Object Reference") (Object :type "StaticMeshComponent Object Reference"))
  (bind _returnvalue (`KismetMaterialLibrary.CreateDynamicMaterialInstance` (`PrimitiveComponent.GetMaterial` Object 0)))
  (`MaterialInstanceDynamic.SetVectorParameterValue` _returnvalue "Pole1" (`KismetMathLibrary.Conv_VectorToLinearColor` (`SceneComponent.K2_GetComponentLocation` Pole0)))
  (`MaterialInstanceDynamic.SetVectorParameterValue` _returnvalue "Pole2" (`KismetMathLibrary.Conv_VectorToLinearColor` (`SceneComponent.K2_GetComponentLocation` Pole1)))
  (`PrimitiveComponent.SetMaterial` Object 0 _returnvalue))

(fn `UserConstructionScript`)