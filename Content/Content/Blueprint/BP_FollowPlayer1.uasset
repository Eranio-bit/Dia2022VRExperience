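; Actor that continuously turns to face the player's VR camera.
; On BeginPlay it caches the player pawn as a MotionControllerPawn, stopping if the cast fails.
; FacePlayer interpolates from the Ochi component's world rotation toward a look-at rotation to the pawn's camera and applies it to the whole actor.
; The event re-calls itself after a very short Delay, acting as an update loop in place of Tick.
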(event `self.ReceiveBeginPlay`
  (bind _asmotion_controller_pawn (cast `/Game/VirtualRealityBP/Blueprints/MotionControllerPawn` (`GameplayStatics.GetPlayerPawn` 0)))
  (set `self.MotionControllerPawn` _asmotion_controller_pawn)
  (`self.Face Player`))

(event `Face Player`
  (bind _ochi (`self.Ochi`))
  ;[1 1 1] Always Face Player
  (`self.K2_SetActorRotation` (`KismetMathLibrary.RInterpTo` (`SceneComponent.K2_GetComponentRotation` _ochi) (`KismetMathLibrary.FindLookAtRotation` (`SceneComponent.K2_GetComponentLocation` _ochi) (`SceneComponent.K2_GetComponentLocation` (`/Game/VirtualRealityBP/Blueprints/MotionControllerPawn.Camera` (`self.MotionControllerPawn`)))) (`GameplayStatics.GetWorldDeltaSeconds`) 1.0))
  (`KismetSystemLibrary.Delay` 0.001)
  (`self.Face Player`))

(fn `UserConstructionScript`)