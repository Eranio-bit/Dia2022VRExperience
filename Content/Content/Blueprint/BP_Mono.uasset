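; BP_Mono is a cart actor, likely a monorail, that rides along the spline of a referenced track.
; On BeginPlay, an active cart starts its move, which plays the CartMover timeline at a rate of one over Duration.
; Each update maps the timeline alpha to a distance along the spline and sets the actor's world location and rotation from that point.
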(event `self.ReceiveBeginPlay`
  (if (`self.ActiveCart`)
    (`self.Move_cart`)))

(event `Move_cart`
  (bind _returnvalue (`KismetMathLibrary.Lerp` 0.0 (`SplineComponent.GetSplineLength` (`/Game/Content/Blueprint/BP_Track.Spline` (`self.TrackRef`))) (`self.Alpha`)))
  (`TimelineComponent.SetPlayRate` (`self.CartMover`) (/ 1.0 (`self.Duration`)))
  (bind (_direction _alpha) (`Timeline|CartMover`)
    (:`Update`
      (set `self.Alpha` _alpha)
      (`self.K2_SetActorLocationAndRotation` (`SplineComponent.GetLocationAtDistanceAlongSpline` (`/Game/Content/Blueprint/BP_Track.Spline` (`self.TrackRef`)) _returnvalue "World") (`SplineComponent.GetRotationAtDistanceAlongSpline` (`/Game/Content/Blueprint/BP_Track.Spline` (`self.TrackRef`)) _returnvalue "World")))))

(fn `UserConstructionScript`)