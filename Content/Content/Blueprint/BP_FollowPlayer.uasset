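; BP_FollowPlayer is an actor that continuously turns to face the player; despite its name, it only rotates and never moves.
; On BeginPlay it caches player 0's ThirdPersonCharacter and starts the FacePlayer event, stopping if the cast fails.
; FacePlayer interpolates the actor's rotation toward the character with RInterpTo, then re-calls itself after a tiny Delay, forming a loop in place of Tick.
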(event `self.ReceiveBeginPlay`
  (bind _asthird_person_character (cast `/Game/ThirdPersonBP/Blueprints/ThirdPersonCharacter` (`GameplayStatics.GetPlayerCharacter` 0)))
  (set `self.Char Ref` _asthird_person_character)
  (`self.Face Player`))

(event `Face Player`
  ;[1 1 1] Always Face Player
  (`self.K2_SetActorRotation` (`KismetMathLibrary.RInterpTo` (`self.K2_GetActorRotation`) (`KismetMathLibrary.FindLookAtRotation` (`self.K2_GetActorLocation`) (`self.K2_GetActorLocation` (`self.Char Ref`))) (`GameplayStatics.GetWorldDeltaSeconds`) 10.0))
  (`KismetSystemLibrary.Delay` 0.001)
  (`self.Face Player`))

(fn `UserConstructionScript`)