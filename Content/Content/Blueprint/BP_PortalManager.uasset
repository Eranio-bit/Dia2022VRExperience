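; Manages a pair of linked portals by positioning their capture components so each mirrors the player camera's view relative to the other portal.
; Every tick, Portal1Update drives Portal2's front and back captures and Portal2Update drives Portal1's.
; Each update applies the rotation delta between the two portal roots, with the destination yaw flipped 180 degrees, to the camera's location and rotation.
; Front and back captures receive identical transforms.
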(event `self.ReceiveTick`
  (params (DeltaSeconds :type "Float (single-precision)"))
  (`self.Portal1_Update`)
  (`self.Portal2_Update`))

(fn `Portal1_Update`
  (locals (NewLocalVar_0 :type "Vector Structure" :default (0.0 0.0 0.0)))
  (bind _defaultsceneroot (`/Game/Content/Blueprint/BP_PortalExit.DefaultSceneRoot` (`self.Portal2`)))
  (bind _defaultsceneroot_2 (`/Game/Content/Blueprint/BP_PortalEnter.DefaultSceneRoot` (`self.Portal1`)))
  (bind _transformcomponent (`PlayerCameraManager.TransformComponent` (`GameplayStatics.GetPlayerCameraManager` 0)))
  (bind (_returnvalue_roll _returnvalue_pitch _returnvalue_yaw) (`KismetMathLibrary.BreakRotator` (`SceneComponent.K2_GetComponentRotation` _defaultsceneroot)))
  (bind _returnvalue (`KismetMathLibrary.NormalizedDeltaRotator` (`KismetMathLibrary.MakeRotator` _returnvalue_roll _returnvalue_pitch (- _returnvalue_yaw 180.0)) (`SceneComponent.K2_GetComponentRotation` _defaultsceneroot_2)))
  (bind _returnvalue_2 (`KismetMathLibrary.ComposeRotators` (`SceneComponent.K2_GetComponentRotation` _transformcomponent) _returnvalue))
  (bind _returnvalue_3 (+ (- (`SceneComponent.K2_GetComponentLocation` _defaultsceneroot) (`KismetMathLibrary.GreaterGreater_VectorRotator` (`SceneComponent.K2_GetComponentLocation` _defaultsceneroot_2) _returnvalue)) (`KismetMathLibrary.GreaterGreater_VectorRotator` (`SceneComponent.K2_GetComponentLocation` _transformcomponent) _returnvalue)))
  (`SceneComponent.K2_SetWorldLocationAndRotation` (`/Game/Content/Blueprint/BP_PortalExit.PortalCapture_Front` (`self.Portal2`)) _returnvalue_3 _returnvalue_2 false false)
  (`SceneComponent.K2_SetWorldLocationAndRotation` (`/Game/Content/Blueprint/BP_PortalExit.PortalCapture_Back` (`self.Portal2`)) _returnvalue_3 _returnvalue_2 false false))

(fn `Portal2_Update`
  (locals (NewLocalVar_0 :type "Vector Structure" :default (0.0 0.0 0.0)))
  (bind _defaultsceneroot (`/Game/Content/Blueprint/BP_PortalExit.DefaultSceneRoot` (`self.Portal2`)))
  (bind _defaultsceneroot_2 (`/Game/Content/Blueprint/BP_PortalEnter.DefaultSceneRoot` (`self.Portal1`)))
  (bind _transformcomponent (`PlayerCameraManager.TransformComponent` (`GameplayStatics.GetPlayerCameraManager` 0)))
  (bind (_returnvalue_roll _returnvalue_pitch _returnvalue_yaw) (`KismetMathLibrary.BreakRotator` (`SceneComponent.K2_GetComponentRotation` _defaultsceneroot_2)))
  (bind _returnvalue (`KismetMathLibrary.NormalizedDeltaRotator` (`KismetMathLibrary.MakeRotator` _returnvalue_roll _returnvalue_pitch (- _returnvalue_yaw 180.0)) (`SceneComponent.K2_GetComponentRotation` _defaultsceneroot)))
  (bind _returnvalue_2 (`KismetMathLibrary.ComposeRotators` (`SceneComponent.K2_GetComponentRotation` _transformcomponent) _returnvalue))
  (bind _returnvalue_3 (+ (- (`SceneComponent.K2_GetComponentLocation` _defaultsceneroot_2) (`KismetMathLibrary.GreaterGreater_VectorRotator` (`SceneComponent.K2_GetComponentLocation` _defaultsceneroot) _returnvalue)) (`KismetMathLibrary.GreaterGreater_VectorRotator` (`SceneComponent.K2_GetComponentLocation` _transformcomponent) _returnvalue)))
  (`SceneComponent.K2_SetWorldLocationAndRotation` (`/Game/Content/Blueprint/BP_PortalEnter.PortalCapture_Front` (`self.Portal1`)) _returnvalue_3 _returnvalue_2 false false)
  (`SceneComponent.K2_SetWorldLocationAndRotation` (`/Game/Content/Blueprint/BP_PortalEnter.PortalCapture_Back` (`self.Portal1`)) _returnvalue_3 _returnvalue_2 false false))

(fn `UserConstructionScript`)